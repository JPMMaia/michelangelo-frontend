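; BP_ApplicationInstance manages the application's top-level UI, switching between the start, login, register and main menus and the editor view.
; InitializeWidgets creates every view's widget up front, then applies the current view.
; SetCurrentView swaps the viewport widget and shows the cursor, using UI-only input for menus and game-and-UI input for the editor.
; Getters expose the current view, the editor widget and the game data singleton's web API.
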(fn GetCurrentView
  (return (Variables|Default|GetCurrentView)))

(fn SetCurrentView
  (params (NewView :type E_View%20Enum))
  (bind _returnvalue (Game|GetPlayerController 0))
  (bind _currentmenu (Variables|Widgets|GetCurrentMenu))
  (Utilities|IsValid _currentmenu
    (:Is%20Valid
      (Widget|RemovefromParent _currentmenu))
    (:Is%20Not%20Valid
      _))
  (bind _output_get (Variables|Default|SetCurrentView NewView))
  (CallFunction|SetCurrentWidget (Utilities|Select :Index _output_get :NewEnumerator0 (Variables|Widgets|GetStartMenu) :NewEnumerator1 (Variables|Widgets|GetLoginMenu) :NewEnumerator2 (Variables|Widgets|GetRegisterMenu) :NewEnumerator3 (Variables|Widgets|GetMainMenu) :NewEnumerator4 (Variables|Widgets|GetEditor)))
  (if (Utilities|Select :Index _output_get :NewEnumerator0 true :NewEnumerator1 true :NewEnumerator2 true :NewEnumerator3 true :NewEnumerator4 false)
    (Input|SetInputModeUIOnly _returnvalue (Utilities|Select :Index _output_get :NewEnumerator0 (Variables|Widgets|GetStartMenu) :NewEnumerator1 (Variables|Widgets|GetLoginMenu) :NewEnumerator2 (Variables|Widgets|GetRegisterMenu) :NewEnumerator3 (Variables|Widgets|GetMainMenu) :NewEnumerator4 (Variables|Widgets|GetEditor)) "DoNotLock")
    (else
      (Input|SetInputModeGameandUI _returnvalue (Utilities|Select :Index _output_get :NewEnumerator0 (Variables|Widgets|GetStartMenu) :NewEnumerator1 (Variables|Widgets|GetLoginMenu) :NewEnumerator2 (Variables|Widgets|GetRegisterMenu) :NewEnumerator3 (Variables|Widgets|GetMainMenu) :NewEnumerator4 (Variables|Widgets|GetEditor)) "DoNotLock" true))))

(fn InitializeWidgets
  (Utilities|FlowControl|Sequence
    (:then_0
      (bind _returnvalue (UserInterface|CreateWidget "/Game/UI/W_StartMenu.W_StartMenu_C"))
      (Variables|Widgets|SetStartMenu _returnvalue))
    (:then_1
      (bind _returnvalue_2 (UserInterface|CreateWidget "/Game/UI/W_LoginMenu.W_LoginMenu_C"))
      (Variables|Widgets|SetLoginMenu _returnvalue_2))
    (:then_2
      (bind _returnvalue_3 (UserInterface|CreateWidget "/Game/UI/W_MainMenu.W_MainMenu_C"))
      (Variables|Widgets|SetMainMenu _returnvalue_3))
    (:then_3
      (bind _returnvalue_4 (UserInterface|CreateWidget "/Game/UI/W_RegisterMenu.W_RegisterMenu_C"))
      (Variables|Widgets|SetRegisterMenu _returnvalue_4))
    (:then_4
      (bind _returnvalue_5 (UserInterface|CreateWidget "/Game/UI/W_Editor.W_Editor_C"))
      (Variables|Widgets|SetEditor _returnvalue_5))
    (:then_5
      (CallFunction|SetCurrentView (Variables|Default|GetCurrentView)))))

(fn SetCurrentWidget
  (params (NewWidget :type User%20Widget%20Object%20Reference))
  (bind _output_get (Variables|Widgets|SetCurrentMenu NewWidget))
  (UserInterface|Viewport|AddtoViewport _output_get 0)
  (Variables|/Script/Engine.PlayerController|SetbShowMouseCursor (Game|GetPlayerController 0) true))

(fn GetWebAPI
  (bind _returnvalue (Class|GameDataSingleton|GetWebAPI (Class|GameDataSingletonLibrary|GetGameDataSingleton)))
  (return _returnvalue))

(fn GetEditorWidget
  (return (Variables|Widgets|GetEditor)))